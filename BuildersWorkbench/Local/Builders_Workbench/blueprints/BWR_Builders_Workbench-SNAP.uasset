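; Builder's Workbench snap Blueprint that adds an overlap check to placement validation for the workbench.
; CanBePlaced runs the parent check first and passes its result and message through when that result is Fail or higher.
; Otherwise it box-traces on Visibility from SnapBox slightly downward, using the box's extent and rotation, returning FailOverlaps on a hit and Success if clear.
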(event EventBeginPlay
  (|CallParentFunction))

(event Collision|EventActorBeginOverlap
  (params (OtherActor :type Actor%20Object%20Reference)))

(event EventTick
  (params (DeltaSeconds :type Float%20%28single-precision%29)))

(fn ConstructionScript
  (|CallParentFunction))

(fn CanbePlaced
  (params (AttachTo :type Buildable%20Base%20Object%20Reference) (InstanceIndex :type Integer))
  (bind _snapbox (Variables|Default|GetSnapBox))
  (bind _returnvalue (Transformation|GetWorldLocation _snapbox))
  (bind (_failedmessage _returnvalue_2) (|CallParentFunction AttachTo InstanceIndex))
  (if (< (Math|Conversions|ToInteger(Byte) _returnvalue_2) (Math|Conversions|ToInteger(Byte) (Utilities|Enum|LiteralenumECanBePlacedResult "Fail")))
    (bind _returnvalue_3 (Collision|BoxTraceByChannel _returnvalue (- _returnvalue "0, 0,4.000000") (Variables|/Script/Engine.BoxComponent|GetBoxExtent _snapbox) (Transformation|GetWorldRotation _snapbox) "TraceTypeQuery1" false 0 "None"))
    (if _returnvalue_3
      (return "" "Fail_Overlaps")
      (else
        (return "" "Success")))
    (else
      (return _failedmessage _returnvalue_2))))